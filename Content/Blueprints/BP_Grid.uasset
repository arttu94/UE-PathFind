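; BP_Grid is a grid actor that visualizes a path through BP_PathNode actors as debug lines.
; Every tick it calls DebugPath on its Finish node, which recursively follows CameFrom links back toward the Start node, drawing a short-lived, raised blue line for each link.
; The recursion ends at a Start-type node, a missing CameFrom or a failed cast.
; The file only displays the path and does not compute it.
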(event `self.ReceiveBeginPlay`)

(event `self.ReceiveTick`
  (params (DeltaSeconds :type "Float (single-precision)"))
  (`self.DebugPath` (`|ConvertAsset` (`self.Finish`))))

(fn `DebugPath`
  (params (InNode :type "GraphSearchNode Soft Object Reference"))
  (returns (OutNode :type "GraphSearchNode Soft Object Reference"))
  (bind _output (`|ConvertAsset` InNode))
  (bind _camefrom (`PathNode.CameFrom` (`|ConvertAsset` InNode)))
  (if (`KismetSystemLibrary.IsValid` _camefrom)
    (`KismetSystemLibrary.DrawDebugLine` (+ (`self.K2_GetActorLocation` _output) (0.0 0.0 60.0)) (+ (`self.K2_GetActorLocation` _camefrom) (0.0 0.0 60.0)) (struct :`G` 0.204077 :`B` 1.0 :`A` 1.0) 0.1 10.0)
    (bind _asbp_path_node (cast `/Game/Blueprints/BP_PathNode` _output))
    (if (`|EnumEquality` (`PathNode.NodeType` _asbp_path_node) "PN_Start")
      (return null)
      (else
        (bind _outnode (`self.DebugPath` (`|ConvertAsset` _camefrom)))
        (return _outnode)))))

(fn `UserConstructionScript`)