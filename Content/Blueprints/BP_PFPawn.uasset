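; BP_PFPawn is the input pawn for a pathfinding demo, triggering search algorithms on a Graph from the keyboard.
; Number keys run breadth-first (with or without an end node), greedy best-first, Dijkstra or A* searches from the graph's start node, while R clears its nodes.
; The searches are called but not defined here, and the HUD widget creation is disconnected, so it never runs.
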(event `self.ReceiveBeginPlay`)

(event `Key|R`
  (params (Key :type "Key Structure"))
  (:`Pressed`
    (`GridGraph.ClearGraphNodes` (`self.Graph`))))

(event `Key|One`
  (params (Key :type "Key Structure"))
  (:`Pressed`
    (`GraphSearch.BreadthFirstSearch` (`GridGraph.Start` (`self.Graph`)))))

(event `Key|Two`
  (params (Key :type "Key Structure"))
  (bind _graph (`self.Graph`))
  (:`Pressed`
    (`GraphSearch.BreadthFirstSearch` (`GridGraph.Start` _graph) (`GridGraph.Finish` _graph))))

(event `Key|Three`
  (params (Key :type "Key Structure"))
  (bind _graph (`self.Graph`))
  (:`Pressed`
    (`GraphSearch.GreedyBestFirstSearch` (`GridGraph.Start` _graph) (`GridGraph.Finish` _graph))))

(event `Key|Four`
  (params (Key :type "Key Structure"))
  (bind _graph (`self.Graph`))
  (:`Pressed`
    (`GraphSearch.DijkstraSearch` (`GridGraph.Start` _graph) (`GridGraph.Finish` _graph))))

(event `Key|Five`
  (params (Key :type "Key Structure"))
  (bind _graph (`self.Graph`))
  (:`Pressed`
    (`GraphSearch.AStarSearch` (`GridGraph.Start` _graph) (`GridGraph.Finish` _graph))))

(fn `UserConstructionScript`)