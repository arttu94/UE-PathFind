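; Free-flying pawn that lets the player paint mNode actors between Open and Closed with the mouse.
; While left mouse is held, a gated Tick traces under the cursor and notifies each newly hit node of its type change.
; The first node's type sets the brush, so the whole stroke applies its opposite.
; Holding right mouse hides the cursor and enables look and move input; releasing restores cursor mode.
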(event `self.ReceiveBeginPlay`
  (bind _returnvalue (`GameplayStatics.GetPlayerController` 0))
  (set `PlayerController.bEnableClickEvents` true _returnvalue)
  (set `PlayerController.bEnableMouseOverEvents` true _returnvalue))

(event `self.ReceiveTick`
  (params (DeltaSeconds :type "Float (single-precision)"))
  (bind _lastmodifyednode (`self.LastModifyedNode`))
  (`/Engine/EditorBlueprintResources/StandardMacros.Gate` true :!label _label
    (:`Exit`
      (bind _outhit (`KismetSystemLibrary.LineTraceSingle` :`Start` (`self.K2_GetActorLocation`) :`End` (+ (`self.K2_GetActorLocation`) (* (`.WorldDirection` (`PlayerController.DeprojectMousePositionToWorld` (`GameplayStatics.GetPlayerController` 0))) 10000.0)) :`TraceChannel` "TraceTypeQuery1" :`DrawTime` 1.0))
      (bind _asm_node (cast `/Game/Blueprints/Pure/mNode` (`.HitActor` (`GameplayStatics.BreakHitResult` _outhit))))
      (if (!= _asm_node (`self.LastModifyedNode`))
        (bind _output_get (set `self.LastModifyedNode` _asm_node))
        (if (not (`|EnumInequality` "NewEnumerator0" (`self.NodeBrushType`)))
          (set `self.NodeBrushType` (`/Game/Blueprints/Pure/mNode.NodeType` _output_get)))
        (switch `/Game/Blueprints/Pure/NodeType` (`self.NodeBrushType`)
          (:`NewEnumerator1`
            (set `/Game/Blueprints/Pure/mNode.NodeType` "NewEnumerator2" _lastmodifyednode)
            (`/Game/Blueprints/Pure/mNode.OnNodeTypeChange` _lastmodifyednode))
          (:`NewEnumerator2`
            (set `/Game/Blueprints/Pure/mNode.NodeType` "NewEnumerator1" _lastmodifyednode)
            (`/Game/Blueprints/Pure/mNode.OnNodeTypeChange` _lastmodifyednode)))))))

(event `Key|LeftMouseButton`
  (params (Key :type "Key Structure"))
  (:`Pressed`
    (goto _label :!via `Open`))
  (:`Released`
    (set `self.LastModifyedNode` null)
    (set `self.NodeBrushType` "NewEnumerator0")
    (goto _label :!via `Close`)))

(event `Key|RightMouseButton`
  (params (Key :type "Key Structure"))
  (bind _returnvalue (`GameplayStatics.GetPlayerController` 0))
  (bind _returnvalue_2 (`GameplayStatics.GetPlayerController` 0))
  (bind _returnvalue_3 (`GameplayStatics.GetPlayerController` 0))
  (bind _returnvalue_4 (`GameplayStatics.GetPlayerController` 0))
  (:`Pressed`
    (`WidgetBlueprintLibrary.SetInputMode_GameOnly` _returnvalue)
    (set `PlayerController.bShowMouseCursor` false _returnvalue_3)
    (`Controller.SetIgnoreLookInput` _returnvalue_2 false)
    (`Controller.SetIgnoreMoveInput` _returnvalue_4 false))
  (:`Released`
    (`WidgetBlueprintLibrary.SetInputMode_GameAndUIEx` _returnvalue null "DoNotLock" false)
    (set `PlayerController.bShowMouseCursor` true _returnvalue_3)
    (`Controller.SetIgnoreLookInput` _returnvalue_2 true)
    (`Controller.SetIgnoreMoveInput` _returnvalue_4 true)))

(event `InputAxis|MoveForward`
  (params (AxisValue :type "Float (single-precision)"))
  ;[1 1 1] Movement
  (`PawnMovementComponent.AddInputVector` (`self.FloatingPawnMovement`) (* (`self.GetActorForwardVector`) AxisValue) false))

(event `InputAxis|MoveRight`
  (params (AxisValue :type "Float (single-precision)"))
  ;[1 1 1] Movement
  (`PawnMovementComponent.AddInputVector` (`self.FloatingPawnMovement`) (* (`self.GetActorRightVector`) AxisValue) false))

(event `InputAxis|CameraPitch`
  (params (AxisValue :type "Float (single-precision)"))
  ;[1 1 1] Camera
  (`self.AddControllerPitchInput` AxisValue))

(event `InputAxis|CameraYaw`
  (params (AxisValue :type "Float (single-precision)"))
  ;[1 1 1] Camera
  (`self.AddControllerYawInput` AxisValue))

(fn `UserConstructionScript`)