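; mNode is a clickable-grid-style node actor that displays itself as either Open or Closed based on its NodeType.
; The OnNodeTypeChange event sets the actor's height, flat for Open and raised for Closed, and swaps the mesh material to match.
; Cursor hover toggles custom depth rendering on the mesh for highlighting, while the click handler is an empty stub.
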(event `OnNodeTypeChange`
  (bind _x (.x (`self.K2_GetActorLocation`)))
  (bind _y (.y (`self.K2_GetActorLocation`)))
  (switch `/Game/Blueprints/Pure/NodeType` (`self.NodeType`)
    (:`NewEnumerator1`
      (`self.K2_SetActorLocation` (`KismetMathLibrary.MakeVector` _x _y))
      (`PrimitiveComponent.SetMaterial` (`self.StaticMesh`) 0 "/Game/Materials/Node_Open.Node_Open"))
    (:`NewEnumerator2`
      (`self.K2_SetActorLocation` (`KismetMathLibrary.MakeVector` _x _y 50.0))
      (`PrimitiveComponent.SetMaterial` (`self.StaticMesh`) 0 "/Game/Materials/Node_Closed.Node_Closed"))))

(event `self.StaticMesh.OnClicked`
  (params (TouchedComponent :type "PrimitiveComponent Object Reference") (ButtonPressed :type "Key Structure")))

(event `self.StaticMesh.OnBeginCursorOver`
  (params (TouchedComponent :type "PrimitiveComponent Object Reference"))
  (`PrimitiveComponent.SetRenderCustomDepth` (`self.StaticMesh`) true))

(event `self.StaticMesh.OnEndCursorOver`
  (params (TouchedComponent :type "PrimitiveComponent Object Reference"))
  (`PrimitiveComponent.SetRenderCustomDepth` (`self.StaticMesh`) false))

(fn `UserConstructionScript`)