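; BP_PathNode is a pathfinding node actor that visualizes the route back to the start through debug drawing.
; Each tick it draws a short red arrow pointing toward its CameFrom node.
; Hovering the cursor enables custom depth and opens a gate, so Tick also calls FindStart.
; FindStart recursively follows CameFrom links, drawing thick blue lines until it returns a Start-type node or one without a valid predecessor.
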(event `self.ReceiveTick`
  (params (DeltaSeconds :type "Float (single-precision)"))
  (`self.DrawCameFromArrow`)
  (`/Engine/EditorBlueprintResources/StandardMacros.Gate` true :!label _label
    (:`Exit`
      (`self.FindStart` self))))

(event `self.StaticMeshComp.OnBeginCursorOver`
  (params (TouchedComponent :type "PrimitiveComponent Object Reference"))
  (`|ExecutionSequence`
    (:`then_0`
      (goto _label :!via `Open`))
    (:`then_1`
      (`PrimitiveComponent.SetRenderCustomDepth` (`self.StaticMeshComp`) true))))

(event `self.StaticMeshComp.OnEndCursorOver`
  (params (TouchedComponent :type "PrimitiveComponent Object Reference"))
  (`|ExecutionSequence`
    (:`then_0`
      (goto _label :!via `Close`))
    (:`then_1`
      (`PrimitiveComponent.SetRenderCustomDepth` (`self.StaticMeshComp`) false))))

(fn `DrawCameFromArrow`
  (bind _returnvalue (`self.K2_GetActorLocation`))
  (bind _camefrom (`self.CameFrom`))
  (bind _returnvalue_2 (`self.K2_GetActorLocation` _camefrom))
  (if (`KismetSystemLibrary.IsValid` _camefrom)
    (`KismetSystemLibrary.DrawDebugArrow` (+ (+ _returnvalue (* (`KismetMathLibrary.Normal` (- _returnvalue _returnvalue_2)) 25.0)) (0.0 0.0 55.0)) (+ (+ _returnvalue (* (`KismetMathLibrary.Normal` (- _returnvalue_2 _returnvalue)) 25.0)) (0.0 0.0 55.0)) 25.0 (struct :`R` 1.0 :`B` 0.009454 :`A` 1.0) 0.1 5.0)))

(fn `FindStart`
  (params (CameFromIn :type "/Game/Blueprints/BP_PathNode Object Reference"))
  (returns (CameFromOut :type "/Game/Blueprints/BP_PathNode Object Reference"))
  (bind _camefrom (`GraphSearchNode.CameFrom` CameFromIn))
  (if (`KismetSystemLibrary.IsValid` (`PathNode.CameFrom` CameFromIn))
    (`KismetSystemLibrary.DrawDebugLine` (+ (`self.K2_GetActorLocation` CameFromIn) (0.0 0.0 60.0)) (+ (`self.K2_GetActorLocation` _camefrom) (0.0 0.0 60.0)) (struct :`G` 0.109327 :`B` 1.0 :`A` 1.0) 0.1 20.0)
    (if (`|EnumInequality` (`PathNode.NodeType` CameFromIn) "PN_Start")
      (bind _asbp_path_node (cast `/Game/Blueprints/BP_PathNode` _camefrom))
      ;[1 1 1] Recursion! :D
      (bind _camefromout (`self.FindStart` _asbp_path_node))
      (return _camefromout)
      (else
        _)))
  (return CameFromIn))

(fn `UserConstructionScript`)